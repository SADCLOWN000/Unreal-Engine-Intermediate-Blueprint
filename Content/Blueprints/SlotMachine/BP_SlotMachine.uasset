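; Slot machine actor that charges the interacting character 50 for a spin when idle and their balance allows it.
; A timeline swings the handle while three wheels start through WheelSituation, the second and third after random delays.
; WheelSituation picks a random track index and plays the timeline matching the shared XRoll variable.
; When the handle finishes, matching wheel rolls set player 0's balance to the pre-spin amount plus 100.
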(event Custom|XROll%20==%200%20or%20360
  (params (SetWheel :type Static%20Mesh%20Component%20Object%20Reference))
  ;[0.1198 0.1027 0] Wheel Situation Events
  (bind (_direction _newtrack_6 _newtrack_8 _newtrack_9) (Timeline|0%20SituationTimeline PlayFromStart)
    (:Update
      (Transformation|SetRelativeRotation SetWheel (Math|Rotator|MakeRotator (Utilities|Select :Index (Variables|Default|GetIndexNO) :Option%200 _newtrack_6 :Option%201 _newtrack_8 :Option%202 _newtrack_9) 0.0 0.0) false false)
      (bind _output_get (Variables|Default|SetRotatorValue (Math|Rotator|MakeRotator (Utilities|Select :Index (Variables|Default|GetIndexNO) :Option%200 _newtrack_6 :Option%201 _newtrack_8 :Option%202 _newtrack_9) 0.0 0.0)))
      (Variables|Default|SetX%20%28Roll%29 (.Roll (Math|Rotator|BreakRotator _output_get))))))

(event Custom|XRoll%20==%20110
  (params (SetWheel :type Static%20Mesh%20Component%20Object%20Reference))
  ;[0.1198 0.1027 0] Wheel Situation Events
  (bind (_direction _newtrack_6 _newtrack_8 _newtrack_9) (Timeline|110%20SituationTimeline PlayFromStart)
    (:Update
      (Transformation|SetRelativeRotation SetWheel (Math|Rotator|MakeRotator (Utilities|Select :Index (Variables|Default|GetIndexNO) :Option%200 _newtrack_6 :Option%201 _newtrack_8 :Option%202 _newtrack_9) 0.0 0.0) false false)
      (bind _output_get (Variables|Default|SetRotatorValue (Math|Rotator|MakeRotator (Utilities|Select :Index (Variables|Default|GetIndexNO) :Option%200 _newtrack_6 :Option%201 _newtrack_8 :Option%202 _newtrack_9) 0.0 0.0)))
      (Variables|Default|SetX%20%28Roll%29 (.Roll (Math|Rotator|BreakRotator _output_get))))))

(event Custom|XRoll%20==%20230
  (params (SetWheel :type Static%20Mesh%20Component%20Object%20Reference))
  ;[0.1198 0.1027 0] Wheel Situation Events
  (bind (_direction _newtrack_6 _newtrack_8 _newtrack_9) (Timeline|230%20SituationTimeline PlayFromStart)
    (:Update
      (Transformation|SetRelativeRotation SetWheel (Math|Rotator|MakeRotator (Utilities|Select :Index (Variables|Default|GetIndexNO) :Option%200 _newtrack_6 :Option%201 _newtrack_8 :Option%202 _newtrack_9) 0.0 0.0) false false)
      (bind _output_get (Variables|Default|SetRotatorValue (Math|Rotator|MakeRotator (Utilities|Select :Index (Variables|Default|GetIndexNO) :Option%200 _newtrack_6 :Option%201 _newtrack_8 :Option%202 _newtrack_9) 0.0 0.0)))
      (Variables|Default|SetX%20%28Roll%29 (.Roll (Math|Rotator|BreakRotator _output_get))))))

(event EventInteractEvent
  (params (CharacterRef :type Character%20Object%20Reference))
  (bind _wheelmesh1 (Variables|Default|GetWheelMesh1))
  (bind _returnvalue (Transformation|GetRelativeTransform _wheelmesh1))
  (bind _roll (Math|Rotator|BreakRotator (.rotation _returnvalue)))
  ;[0.1354 0.1163 0] Spen Money on Slot Machine
  (if (not (Variables|Default|GetisWorking?))
    (bind _money (Class|BPICharacter|GetCurrentBalance(Message) CharacterRef))
    (if (>= _money 50)
      (Class|BPICharacter|UpdateBalance(Message) CharacterRef (- _money 50))
      (Utilities|FlowControl|Sequence
        (:then_0
          (bind _newtrack_0 (Timeline|MoveHandleTimeline PlayFromStart)
            (:Update
              (Variables|Default|SetisWorking? true)
              (Transformation|SetRelativeRotation (Variables|Default|GetHandleMesh) (Math|Rotator|MakeRotator _newtrack_0 0.0 0.0) false false))
            (:Finished
              (Variables|Default|SetisWorking? false)
              ;[0.1354 0.1163 0] Get 100$ for Each Win
              (if (and (== (.Roll (Math|Rotator|BreakRotator (.rotation (Transformation|GetRelativeTransform (Variables|Default|GetWheelMesh0))))) _roll) (== _roll (.Roll (Math|Rotator|BreakRotator (.rotation (Transformation|GetRelativeTransform (Variables|Default|GetWheelMesh2)))))))
                (Class|BPICharacter|UpdateBalance(Message) (Game|GetPlayerCharacter 0) (+ _money 100))))))
        (:then_1
          (CallFunction|WheelSituation (Variables|Default|GetWheelMesh0)))
        (:then_2
          (Utilities|FlowControl|Delay (Math|Random|RandomFloatinRange 0.0 0.6))
          (CallFunction|WheelSituation (Variables|Default|GetWheelMesh1)))
        (:then_3
          (Utilities|FlowControl|Delay (Math|Random|RandomFloatinRange 0.5 1.0))
          (CallFunction|WheelSituation (Variables|Default|GetWheelMesh2)))))))

(fn ConstructionScript)

(fn WheelSituation
  (params (GetWheel :type Static%20Mesh%20Component%20Object%20Reference))
  (Variables|Default|SetIndexNO (Math|Random|RandomInteger 2))
  ;[0.04355 0.04621 0.2656] XRoll == 0 or 360
  (Utilities|FlowControl|Sequence
    (:then_0
      (if (or (== (Variables|Default|GetX%20%28Roll%29) 0.0) (== (Variables|Default|GetX%20%28Roll%29) 3.6e+02))
        (Variables|Default|SetX%20%28Roll%29 0.0)
        (CallFunction|XROll==0or360 GetWheel)))
    (:then_1
      ;[0 0.265 0.401] XRoll == 110
      (if (== (Variables|Default|GetX%20%28Roll%29) 1.1e+02)
        (CallFunction|XRoll==110 GetWheel)))
    (:then_2
      ;[0.5729 0.1717 0.3748] XRoll == 230
      (if (== (Variables|Default|GetX%20%28Roll%29) 2.3e+02)
        (CallFunction|XRoll==230 GetWheel)))))